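; BP_CharacterBase is a character pawn Blueprint that handles two debug-style key bindings for UI and combat.
; Tab opens the main battle screen through the UI subsystem.
; Q asks the Ability System Component to activate melee abilities by gameplay tag and prints whether that succeeded.
; Unconnected leftover nodes experiment with Gameplay Task delay and actor spawning, plus a data table row lookup, and never run.
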(event EventBeginPlay)

(event Collision|EventActorBeginOverlap
  (params (OtherActor :type Actor%20Object%20Reference)))

(event EventTick
  (params (DeltaSeconds :type Float%20%28single-precision%29)))

(event Input|KeyboardEvents|Q
  (params (Key :type Key%20Structure :default "None"))
  (:Pressed
    (bind _returnvalue (Abilities|TryActivateAbilitiesbyTag (Variables|Default|GetAbilitySystemComponent) (Variables|Default|GetAbility_Melee) true))
    (Development|PrintString (Utilities|String|ToString(Boolean) _returnvalue))))

(event Input|KeyboardEvents|Tab
  (params (Key :type Key%20Structure :default "None"))
  (:Pressed
    (Class|UISubsystem|Open (Subsystems|GetUISubsystem) "UIBattleMain")))

(fn ConstructionScript)